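; AI controller logic for a computer player in the frog feeding minigame, deciding which pea throw to make.
; On possession it caches the BP_FrogFeedingPlayer, then every tick switches on that player's Size to pick randomly between two of the light, medium and heavy throws.
; If a pea is ready it throws after a short delay, randomized for some branches and fixed for others, without rechecking readiness afterwards.
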(event `self.OnMinigamePlayerPossessed`
  (bind _asbp_frog_feeding_player (cast `/Game/BP_FrogFeedingPlayer` (`self.Player`)))
  (set `self.As BP Frog Feeding Player` _asbp_frog_feeding_player))

(event `self.ReceiveTick`
  (params (DeltaSeconds :type "Float (single-precision)"))
  (bind _returnvalue (== (`self.Random`) 1))
  (bind _peaready (`/Game/BP_FrogFeedingPlayer.PeaReady` (`self.As BP Frog Feeding Player`)))
  (bind _peaready_2 (`/Game/BP_FrogFeedingPlayer.PeaReady` (`self.As BP Frog Feeding Player`)))
  (bind _peaready_3 (`/Game/BP_FrogFeedingPlayer.PeaReady` (`self.As BP Frog Feeding Player`)))
  (set `self.Random` (`KismetMathLibrary.RandomInteger` 2))
  (set `self.DelayBeforeThrow` (`KismetMathLibrary.RandomFloatInRange` 0.2 1.0))
  (switch `int` (`/Game/BP_FrogFeedingPlayer.Size` (`self.As BP Frog Feeding Player`))
    (:`0`
      ; Light throw
      (if _returnvalue
        (if _peaready
          (`KismetSystemLibrary.Delay` (`self.DelayBeforeThrow`))
          (`/Game/BP_FrogFeedingPlayer.LightThrow` (`self.As BP Frog Feeding Player`)))
        (else
          ; Medium throw
          (if _peaready
            (`KismetSystemLibrary.Delay` (`self.DelayBeforeThrow`))
            (`/Game/BP_FrogFeedingPlayer.Medium Throw` (`self.As BP Frog Feeding Player`))))))
    (:`1`
      (if _returnvalue
        (if _peaready_2
          (`KismetSystemLibrary.Delay` (`self.DelayBeforeThrow`))
          (`/Game/BP_FrogFeedingPlayer.Medium Throw` (`self.As BP Frog Feeding Player`)))
        (else
          ; Heavy throw
          (if _peaready_2
            (`KismetSystemLibrary.Delay` 0.2)
            (`/Game/BP_FrogFeedingPlayer.HeavyThrow` (`self.As BP Frog Feeding Player`))))))
    (:`2`
      (if _returnvalue
        (if _peaready_3
          (`KismetSystemLibrary.Delay` 0.2)
          (`/Game/BP_FrogFeedingPlayer.HeavyThrow` (`self.As BP Frog Feeding Player`)))
        (else
          ; Light throw
          (if _peaready_3
            (`KismetSystemLibrary.Delay` 0.2)
            (`/Game/BP_FrogFeedingPlayer.LightThrow` (`self.As BP Frog Feeding Player`))))))))

(fn `UserConstructionScript`)